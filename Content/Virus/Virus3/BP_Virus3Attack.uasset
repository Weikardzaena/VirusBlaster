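; BP_Virus3Attack is the attack actor of the third virus enemy, damaging BP_Ship actors on contact.
; A blocking hit damages a ship and destroys the actor whatever it struck, while a sphere overlap damages and self-destructs only for ships.
; Both paths apply the Damage variable, crediting the instigator's AI controller as the event instigator.
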(event `self.ReceiveHit`
  (params (MyComp :type "PrimitiveComponent Object Reference") (Other :type "Actor Object Reference") (OtherComp :type "PrimitiveComponent Object Reference") (bSelfMoved :type Boolean) (HitLocation :type "Vector Structure") (HitNormal :type "Vector Structure") (NormalImpulse :type "Vector Structure") (Hit :type "HitResult Structure (by ref)"))
  (bind _asbp_ship (cast `/Game/FirstPersonBP/Blueprints/BP_Ship` Other)
    (:`then`
      (`GameplayStatics.ApplyDamage` _asbp_ship (`self.Damage`) (`AIBlueprintHelperLibrary.GetAIController` (`self.GetInstigator`)) self))
    (:`CastFailed`
      _))
  (`self.K2_DestroyActor`))

(event `self.SphereCollision.OnComponentBeginOverlap`
  (params (OverlappedComponent :type "PrimitiveComponent Object Reference") (OtherActor :type "Actor Object Reference") (OtherComp :type "PrimitiveComponent Object Reference") (OtherBodyIndex :type Integer) (bFromSweep :type Boolean) (SweepResult :type "HitResult Structure (by ref)"))
  (bind _asbp_ship (cast `/Game/FirstPersonBP/Blueprints/BP_Ship` OtherActor))
  (`GameplayStatics.ApplyDamage` _asbp_ship (`self.Damage`) (`AIBlueprintHelperLibrary.GetAIController` (`self.GetInstigator`)) self)
  (`self.K2_DestroyActor`))

(fn `UserConstructionScript`)