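; Base Blueprint for the Virus-2 enemy, which turns to face the player ship within range and shoots at it.
; Detection sphere overlaps toggle a lock-on flag, and while locked, Tick snaps the root's rotation toward the ship.
; A looping timer traces forward on the Camera channel as far as the sphere's radius.
; If that trace hits the ship, it spawns a VirusAttack carrying the virus's attack damage.
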(event `OnEnterDetectionRadius`
  (params (OverlappedComponent :type "PrimitiveComponent Object Reference") (OtherActor :type "Actor Object Reference") (OtherComp :type "PrimitiveComponent Object Reference") (OtherBodyIndex :type Integer) (bFromSweep :type Boolean) (SweepResult :type "HitResult Structure (by ref)"))
  (cast `/Game/FirstPersonBP/Blueprints/BP_Ship` OtherActor)
  (set `self.IsLockedOn` true))

(event `self.ReceiveBeginPlay`
  (`parent.ReceiveBeginPlay`)
  (`|ExecutionSequence`
    (:`then_0`
      (add `PrimitiveComponent.OnComponentBeginOverlap` (`self.DetectionSphere`) (delegate `OnEnterDetectionRadius`)))
    (:`then_1`
      (add `PrimitiveComponent.OnComponentEndOverlap` (`self.DetectionSphere`) (delegate `OnLeaveDetectionRadius`)))
    (:`then_2`
      (set `self.IsLockedOn` (`PrimitiveComponent.IsOverlappingActor` (`self.DetectionSphere`) (`self.BPShip`))))
    (:`then_3`
      (`KismetSystemLibrary.K2_SetTimer` self "FireForward" (`self.FirePeriod`) true))))

(event `OnLeaveDetectionRadius`
  (params (OverlappedComponent :type "PrimitiveComponent Object Reference") (OtherActor :type "Actor Object Reference") (OtherComp :type "PrimitiveComponent Object Reference") (OtherBodyIndex :type Integer))
  (cast `/Game/FirstPersonBP/Blueprints/BP_Ship` OtherActor)
  (set `self.IsLockedOn` false))

(event `self.ReceiveTick`
  (params (DeltaSeconds :type "Float (single-precision)"))
  (`parent.ReceiveTick` DeltaSeconds)
  (if (`self.IsLockedOn`)
    (`SceneComponent.K2_SetWorldRotation` (`self.RootComponent`) (`KismetMathLibrary.FindLookAtRotation` (`SceneComponent.K2_GetComponentLocation` (`self.RootComponent`)) (`SceneComponent.K2_GetComponentLocation` (`Actor.RootComponent` (`self.BPShip`)))) false false)))

(fn `FireForward`
  (bind _rootcomponent (`self.RootComponent`))
  (bind _returnvalue (`SceneComponent.K2_GetComponentLocation` _rootcomponent))
  (bind (_outhit _returnvalue_2) (`KismetSystemLibrary.LineTraceSingle` _returnvalue (+ _returnvalue (* (`SceneComponent.GetForwardVector` _rootcomponent) (`SphereComponent.SphereRadius` (`self.DetectionSphere`)))) "TraceTypeQuery2"))
  (if _returnvalue_2
    (if (== (`self.BPShip`) (`.HitActor` (`GameplayStatics.BreakHitResult` _outhit)))
      (`|SpawnActorFromClass` "/Game/Virus/VirusAttack.VirusAttack_C" (`SceneComponent.K2_GetComponentToWorld` (`self.RootComponent`)) "Undefined" "OverrideRootScale" null (`self.GetAttackDamage`) self))))

(fn `UserConstructionScript`
  (`parent.UserConstructionScript`))