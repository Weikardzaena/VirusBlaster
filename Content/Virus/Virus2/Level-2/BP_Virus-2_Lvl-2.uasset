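; Level 2 variant of the Virus 2 enemy character, built on a parent virus Blueprint that it calls for begin play, tick and damage.
; It sets its own death sound and switches walk speed every tick between fast and slow based on IsMoving.
; Overlaps on its Vision component toggle the isThreat Blackboard key on its AI controller, making the virus chase the player.
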(event `self.ReceiveBeginPlay`
  (`parent.ReceiveBeginPlay`)
  (set `self.deathSong` "/Game/Virus/virus2Death.virus2Death"))

(event `self.ReceiveTick`
  (params (DeltaSeconds :type "Float (single-precision)"))
  (bind _charactermovement (`self.CharacterMovement`))
  (`parent.ReceiveTick` DeltaSeconds)
  (if (`self.isMoving`)
    (set `CharacterMovementComponent.MaxWalkSpeed` 350.0 _charactermovement)
    (else
      (set `CharacterMovementComponent.MaxWalkSpeed` 150.0 _charactermovement))))

(event `self.ReceiveAnyDamage`
  (params (Damage :type "Float (single-precision)") (DamageType :type "DamageType Object Reference") (InstigatedBy :type "Controller Object Reference") (DamageCauser :type "Actor Object Reference"))
  (`parent.ReceiveAnyDamage` Damage DamageType InstigatedBy DamageCauser))

(event `self.vision.OnComponentBeginOverlap`
  (params (OverlappedComponent :type "PrimitiveComponent Object Reference") (OtherActor :type "Actor Object Reference") (OtherComp :type "PrimitiveComponent Object Reference") (OtherBodyIndex :type Integer) (bFromSweep :type Boolean) (SweepResult :type "HitResult Structure (by ref)"))
  (bind _returnvalue (`AIBlueprintHelperLibrary.GetBlackboard` (`AIBlueprintHelperLibrary.GetAIController` self)))
  ;[1 1 1] Makes virus chase player
  (if (`KismetSystemLibrary.IsValid` _returnvalue)
    (`BlackboardComponent.SetValueAsBool` _returnvalue "isThreat" true)))

(event `self.vision.OnComponentEndOverlap`
  (params (OverlappedComponent :type "PrimitiveComponent Object Reference") (OtherActor :type "Actor Object Reference") (OtherComp :type "PrimitiveComponent Object Reference") (OtherBodyIndex :type Integer))
  (bind _returnvalue (`AIBlueprintHelperLibrary.GetBlackboard` (`AIBlueprintHelperLibrary.GetAIController` self)))
  ;[1 1 1] Makes virus chase player
  (if (`KismetSystemLibrary.IsValid` _returnvalue)
    (`BlackboardComponent.SetValueAsBool` _returnvalue "isThreat" false)))

(fn `UserConstructionScript`
  (`parent.UserConstructionScript`))