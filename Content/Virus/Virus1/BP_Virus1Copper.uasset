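; BP_Virus1Copper is a Virus1 enemy that chases the player's ship when it comes within sight.
; Overlaps on the Vision1 component set the AI Blackboard target to the ship and clear it on exit.
; BeginPlay also checks for a ship already inside Vision1 and assigns the Virus1 death sound.
; Tick, damage and construction only forward to the parent class.
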(event `self.ReceiveBeginPlay`
  (`parent.ReceiveBeginPlay`)
  (set `self.deathSong` "/Game/Virus/Virus1/virus1Death.virus1Death")
  (if (> (`KismetArrayLibrary.Array_Length` (`PrimitiveComponent.GetOverlappingActors` (`self.vision1`) "/Game/FirstPersonBP/Blueprints/BP_Ship.BP_Ship_C")) 0)
    (if (`self.HasValidBlackboard`)
      (`BlackboardComponent.SetValueAsObject` (`self.GetBlackboard`) (`self.NAME_BB_TARGET`) (`self.BPShip`)))))

(event `self.vision1.OnComponentBeginOverlap`
  (params (OverlappedComponent :type "PrimitiveComponent Object Reference") (OtherActor :type "Actor Object Reference") (OtherComp :type "PrimitiveComponent Object Reference") (OtherBodyIndex :type Integer) (bFromSweep :type Boolean) (SweepResult :type "HitResult Structure (by ref)"))
  ;[1 1 1] Makes virus chase player
  (if (and (`self.HasValidBlackboard`) (== OtherActor (`self.BPShip`)))
    (`BlackboardComponent.SetValueAsObject` (`self.GetBlackboard`) (`self.NAME_BB_TARGET`) (`self.BPShip`))))

(event `self.ReceiveTick`
  (params (DeltaSeconds :type "Float (single-precision)"))
  (`parent.ReceiveTick` DeltaSeconds))

(event `self.vision1.OnComponentEndOverlap`
  (params (OverlappedComponent :type "PrimitiveComponent Object Reference") (OtherActor :type "Actor Object Reference") (OtherComp :type "PrimitiveComponent Object Reference") (OtherBodyIndex :type Integer))
  ;[1 1 1] Makes virus chase player
  (if (and (== (`self.BPShip`) OtherActor) (`self.HasValidBlackboard`))
    (`BlackboardComponent.ClearValue` (`self.GetBlackboard`) (`self.NAME_BB_TARGET`))))

(event `self.ReceiveAnyDamage`
  (params (Damage :type "Float (single-precision)") (DamageType :type "DamageType Object Reference") (InstigatedBy :type "Controller Object Reference") (DamageCauser :type "Actor Object Reference"))
  (`parent.ReceiveAnyDamage` Damage DamageType InstigatedBy DamageCauser))

(fn `UserConstructionScript`
  (`parent.UserConstructionScript`))