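; Base virus enemy that damages the player's ship on contact and tracks its own health.
; It shows a widget health bar that turns each tick to face the ship's camera and updates when damage is taken.
; At zero health it registers the kill with the game state, then swaps its visible body for a destructible mesh that fractures with an outward radial force before the actor is destroyed.
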(event `self.ReceiveBeginPlay`
  (bind _ascustom_game_state (cast `/Game/Game/CustomGameState` (`GameplayStatics.GetGameState`)))
  (set `self.GameState` _ascustom_game_state)
  (bind _asbp_ship (cast `/Game/FirstPersonBP/Blueprints/BP_Ship` (`Controller.K2_GetPawn` (`GameplayStatics.GetPlayerController` 0))))
  (set `self.BPShip` _asbp_ship)
  ;[1 1 1] Initialize the Health Bar
  (bind _returnvalue (`|CreateWidget` "/Game/Virus/HealthWidget.HealthWidget_C"))
  (`/Game/Virus/HealthWidget.SetWidgetStartHealth` _returnvalue (`self.Health`))
  (`WidgetComponent.SetWidget` (`self.HealthWidget`) _returnvalue))

(event `self.DestructibleMesh.OnComponentHit`
  (params (HitComponent :type "PrimitiveComponent Object Reference") (OtherActor :type "Actor Object Reference") (OtherComp :type "PrimitiveComponent Object Reference") (NormalImpulse :type "Vector Structure") (Hit :type "HitResult Structure (by ref)"))
  ;[1 1 1] Deal damage if destructible mesh hits ship
  (bind _asbp_ship (cast `/Game/FirstPersonBP/Blueprints/BP_Ship` OtherActor))
  (`GameplayStatics.ApplyDamage` _asbp_ship (`self.AttackDamage`) (`AIBlueprintHelperLibrary.GetAIController` self) self))

(event `self.DestructibleMesh.OnComponentBeginOverlap`
  (params (OverlappedComponent :type "PrimitiveComponent Object Reference") (OtherActor :type "Actor Object Reference") (OtherComp :type "PrimitiveComponent Object Reference") (OtherBodyIndex :type Integer) (bFromSweep :type Boolean) (SweepResult :type "HitResult Structure (by ref)"))
  ;[1 1 1] Deal damage if destructible mesh overlaps ship
  (bind _asbp_ship (cast `/Game/FirstPersonBP/Blueprints/BP_Ship` OtherActor))
  (`GameplayStatics.ApplyDamage` _asbp_ship (`self.AttackDamage`) (`AIBlueprintHelperLibrary.GetAIController` self) self))

(event `self.ReceiveTick`
  (params (DeltaSeconds :type "Float (single-precision)"))
  (bind _healthwidget (`self.HealthWidget`))
  ;[1 1 1] Turn health bar towards player
  (`SceneComponent.K2_SetWorldRotation` _healthwidget (`KismetMathLibrary.FindLookAtRotation` (`SceneComponent.K2_GetComponentLocation` _healthwidget) (`SceneComponent.K2_GetComponentLocation` (`/Game/FirstPersonBP/Blueprints/BP_Ship.PrimaryCamera` (`self.BPShip`)))) false false))

(event `self.ReceiveAnyDamage`
  (params (Damage :type "Float (single-precision)") (DamageType :type "DamageType Object Reference") (InstigatedBy :type "Controller Object Reference") (DamageCauser :type "Actor Object Reference"))
  (bind _destructiblemesh (`self.DestructibleMesh`))
  (bind _capsulecomponent (`self.CapsuleComponent`))
  (bind _returnvalue (`SceneComponent.K2_GetComponentLocation` _destructiblemesh))
  ;[1 1 1] Subtract health from virus
  (if (not (`self.IsDying`))
    (bind _output_get (set `self.Health` (`KismetMathLibrary.FMax` (- (`self.Health`) Damage))))
    ;[1 1 1] Update Health Bar
    (bind _ashealth_widget (cast `/Game/Virus/HealthWidget` (`WidgetComponent.GetUserWidgetObject` (`self.HealthWidget`)))
      (:`then`
        (`/Game/Virus/HealthWidget.SetWidgetHealth` _ashealth_widget _output_get))
      (:`CastFailed`
        _))
    ;[1 1 1] If dead, perform destructible mesh stuff
    (if (`KismetMathLibrary.NearlyEqual_FloatFloat` _output_get)
      (set `self.IsDying` true)
      (`/Game/Game/CustomGameState.RegisterVirusKill` (`self.GameState`) self)
      ;[1 1 1] Turn primary mesh invisible and disable collision
      (if (`KismetSystemLibrary.IsValid` (`self.DestructibleMesh`))
        (`SceneComponent.SetVisibility` _capsulecomponent false true)
        (`PrimitiveComponent.SetCollisionEnabled` _capsulecomponent "NoCollision")
        ;[1 1 1] Make destructible mesh visible
        (`SceneComponent.SetVisibility` _destructiblemesh true true)
        ;[1 1 1] Fracture destructible mesh and wait for destroy
        (`DestructibleComponent.ApplyDamage` _destructiblemesh 1.0 _returnvalue _returnvalue 1.0)
        (`KismetSystemLibrary.Delay` 2.0))
      (`self.K2_DestroyActor`))))

(event `self.ReceiveHit`
  (params (MyComp :type "PrimitiveComponent Object Reference") (Other :type "Actor Object Reference") (OtherComp :type "PrimitiveComponent Object Reference") (bSelfMoved :type Boolean) (HitLocation :type "Vector Structure") (HitNormal :type "Vector Structure") (NormalImpulse :type "Vector Structure") (Hit :type "HitResult Structure (by ref)"))
  ;[1 1 1] If we hit the player, deal damage to them
  (bind _asbp_ship (cast `/Game/FirstPersonBP/Blueprints/BP_Ship` Other))
  (`GameplayStatics.ApplyDamage` _asbp_ship (`self.AttackDamage`) (`AIBlueprintHelperLibrary.GetAIController` self) self))

(event `self.DestructibleMesh.OnComponentFracture`
  (params (HitPoint :type "Vector Structure (by ref)") (HitDirection :type "Vector Structure (by ref)"))
  (bind _destructiblemesh (`self.DestructibleMesh`))
  ;[1 1 1] Explode fractured pieces outward radially from center
  (`PrimitiveComponent.AddRadialForce` _destructiblemesh (`SceneComponent.K2_GetComponentLocation` _destructiblemesh) 100.0 50000.0 "RIF_Constant" true))

(fn `GetAttackDamage`
  (returns (AttackDamageVal :type "Float (double-precision)"))
  (return (`self.AttackDamage`)))

(fn `UserConstructionScript`)