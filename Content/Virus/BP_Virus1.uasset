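; BP_Virus1 is a virus character Blueprint that specializes a parent class with its own death sound and movement speeds.
; On BeginPlay it runs the parent logic, then assigns Virus1Death as DeathSong.
; Each Tick sets the max walk speed to a faster or slower value based on IsMoving.
; Damage and construction logic simply defer to the parent.
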(event `self.ReceiveBeginPlay`
  (`parent.ReceiveBeginPlay`)
  (set `self.deathSong` "/Game/Virus/virus1Death.virus1Death"))

(event `self.ReceiveTick`
  (params (DeltaSeconds :type "Float (single-precision)"))
  (bind _charactermovement (`self.CharacterMovement`))
  (`parent.ReceiveTick` DeltaSeconds)
  (if (`self.isMoving`)
    (set `CharacterMovementComponent.MaxWalkSpeed` 350.0 _charactermovement)
    (else
      (set `CharacterMovementComponent.MaxWalkSpeed` 150.0 _charactermovement))))

(event `self.ReceiveAnyDamage`
  (params (Damage :type "Float (single-precision)") (DamageType :type "DamageType Object Reference") (InstigatedBy :type "Controller Object Reference") (DamageCauser :type "Actor Object Reference"))
  (`parent.ReceiveAnyDamage` Damage DamageType InstigatedBy DamageCauser))

(fn `UserConstructionScript`
  (`parent.UserConstructionScript`))