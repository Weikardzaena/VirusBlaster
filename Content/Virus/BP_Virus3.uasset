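; BP_Virus3 is a virus enemy that periodically fires attacks at the player when within aggro range.
; On BeginPlay it caches the player character and starts a looping AttackPlayer timer at the attack period.
; Each attack checks capsule-to-capsule distance, then spawns a BP_Virus3Attack rotated toward the player, passing damage and itself as owner and instigator.
; BeginPlay, Tick, damage and construction defer to the parent class.
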(event `self.ReceiveBeginPlay`
  (`parent.ReceiveBeginPlay`)
  (set `self.ThePlayer` (`GameplayStatics.GetPlayerCharacter` 0))
  (`KismetSystemLibrary.K2_SetTimer` null "AttackPlayer" (`self.AttackPeriod`) true))

(event `self.ReceiveTick`
  (params (DeltaSeconds :type "Float (single-precision)"))
  (`parent.ReceiveTick` DeltaSeconds))

(event `self.ReceiveAnyDamage`
  (params (Damage :type "Float (single-precision)") (DamageType :type "DamageType Object Reference") (InstigatedBy :type "Controller Object Reference") (DamageCauser :type "Actor Object Reference"))
  (`parent.ReceiveAnyDamage` Damage DamageType InstigatedBy DamageCauser))

(fn `AttackPlayer`
  (locals (VirusPosition :type "Vector Structure" :default (0.0 0.0 0.0)) (PlayerPosition :type "Vector Structure" :default (0.0 0.0 0.0)))
  (bind _theplayer (`self.ThePlayer`))
  (if (`KismetSystemLibrary.IsValid` _theplayer)
    (bind _output_get (set `local.VirusPosition` (`SceneComponent.K2_GetComponentLocation` (`self.CapsuleComponent`))))
    (bind _output_get_2 (set `local.PlayerPosition` (`SceneComponent.K2_GetComponentLocation` (`Character.CapsuleComponent` _theplayer))))
    (if (< (`KismetMathLibrary.VSize` (- _output_get _output_get_2)) (`self.AggroDistance`))
      (`|SpawnActorFromClass` "/Game/Virus/Virus3/BP_Virus3Attack.BP_Virus3Attack_C" (`KismetMathLibrary.MakeTransform` (`local.VirusPosition`) (`KismetMathLibrary.FindLookAtRotation` (`local.VirusPosition`) (`local.PlayerPosition`))) "Undefined" "OverrideRootScale" self (`self.AttackDamage`) self))))

(fn `UserConstructionScript`
  (`parent.UserConstructionScript`))