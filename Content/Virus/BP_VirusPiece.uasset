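; BP_VirusPiece is a virus fragment projectile that damages player ships on contact.
; It picks a random direction at BeginPlay, and Activate later unhides it, enables sphere physics and collision, and launches it that way.
; Overlapping or hitting a BP_Ship applies damage credited to the virus controller and destroys the piece.
; Otherwise, a timer started on activation destroys it when its lifetime expires.
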(event `self.ReceiveBeginPlay`
  (set `self.InitialDirection` (`KismetMathLibrary.MakeVector` (`KismetMathLibrary.RandomFloatInRange` -1.0 1.0) (`KismetMathLibrary.RandomFloatInRange` -1.0 1.0) (`KismetMathLibrary.RandomFloatInRange` -1.0 1.0)))
  (if (<= (`self.Lifetime`) 0.0)
    (set `self.Lifetime` 1.0)))

(event `self.ReceiveActorBeginOverlap`
  (params (OtherActor :type "Actor Object Reference"))
  (bind _asbp_ship (cast `/Game/FirstPersonBP/Blueprints/BP_Ship` OtherActor))
  (`GameplayStatics.ApplyDamage` _asbp_ship (`self.Damage`) (`self.VirusController`) (`self.GetInstigator`))
  (`self.DestroySelf`))

(event `self.ReceiveHit`
  (params (MyComp :type "PrimitiveComponent Object Reference") (Other :type "Actor Object Reference") (OtherComp :type "PrimitiveComponent Object Reference") (bSelfMoved :type Boolean) (HitLocation :type "Vector Structure") (HitNormal :type "Vector Structure") (NormalImpulse :type "Vector Structure") (Hit :type "HitResult Structure (by ref)"))
  (bind _asbp_ship (cast `/Game/FirstPersonBP/Blueprints/BP_Ship` Other))
  (`GameplayStatics.ApplyDamage` _asbp_ship (`self.Damage`) (`self.VirusController`) (`self.GetInstigator`))
  (`KismetSystemLibrary.PrintString` "Piece hit player and destroy self!")
  (`self.DestroySelf`))

(fn `Activate`
  (bind _spherecollision (`self.SphereCollision`))
  (`PrimitiveComponent.SetSimulatePhysics` _spherecollision true)
  (`PrimitiveComponent.SetCollisionEnabled` _spherecollision "QueryAndPhysics")
  (`PrimitiveComponent.SetCollisionProfileName` _spherecollision (`self.NAME_VIRUS_PROJECTILE`))
  (`PrimitiveComponent.SetPhysicsLinearVelocity` (`self.SphereCollision`) (* (`self.InitialDirection`) (`self.InitialSpeed`)) true "None")
  (`self.SetActorHiddenInGame` false)
  (`KismetSystemLibrary.K2_SetTimer` self "DestroySelf" (`self.Lifetime`)))

(fn `DestroySelf`
  (`self.K2_DestroyActor`))

(fn `UserConstructionScript`)