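; BP_LevelBeginGate is a level-start gate that closes behind the player's ship.
; When a BP_Ship stops overlapping its Box trigger, it records its location and a target lowered along Z by Distance.
; ClosingTimeline then lerps the whole actor between those points without sweeping.
; A Finished flag, set only when the timeline completes, blocks later triggers.
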(event `self.ReceiveBeginPlay`
  (add `PrimitiveComponent.OnComponentEndOverlap` (`self.Box`) (delegate `OnComponentEndOverlap_Trigger`)))

(event `OnComponentEndOverlap_Trigger`
  (params (OverlappedComponent :type "PrimitiveComponent Object Reference") (OtherActor :type "Actor Object Reference") (OtherComp :type "PrimitiveComponent Object Reference") (OtherBodyIndex :type Integer))
  (bind _returnvalue (`self.K2_GetActorLocation`))
  (if (not (`self.Finished`))
    (cast `/Game/FirstPersonBP/Blueprints/BP_Ship` OtherActor)
    (set `self.StartingLocation` _returnvalue)
    (set `self.EndingLocation` (+ _returnvalue (`KismetMathLibrary.MakeVector` 0.0 0.0 (* (`self.Distance`) -1.0))))
    ;[1 1 1] linearly interpolate from the starting position to the ending position
    (bind (_direction _closing_track) (`Timeline|Closing Timeline` :!via `PlayFromStart`)
      (:`Update`
        (`self.K2_SetActorLocation` (`KismetMathLibrary.VLerp` (`self.StartingLocation`) (`self.EndingLocation`) _closing_track)))
      (:`Finished`
        (set `self.Finished` true)))))

(fn `UserConstructionScript`)