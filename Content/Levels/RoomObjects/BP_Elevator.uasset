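; BP_Elevator is a one-shot room elevator that carries the player's BP_Ship down its local Z axis.
; A trigger box overlap stores the ship, disables its input and starts the move.
; Tick eases the ship's rotation toward the elevator's and offsets both actors along their own local down axes.
; Once the accumulated travel reaches VerticalDistance, it stops, restores input and turns off its point light.
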(event `self.ReceiveTick`
  (params (DeltaSeconds :type "Float (single-precision)"))
  (bind _returnvalue (* DeltaSeconds (`self.TravelSpeed`)))
  (bind _returnvalue_2 (`KismetMathLibrary.MakeVector` 0.0 0.0 (* _returnvalue -1.0)))
  (if (and (`self.PlayerInside`) (not (`self.IsFinishedMove`)))
    (`SceneComponent.K2_SetWorldRotation` (`Actor.RootComponent` (`self.Ship`)) (`KismetMathLibrary.RInterpTo` (`self.K2_GetActorRotation` (`self.Ship`)) (`SceneComponent.K2_GetComponentRotation` (`self.RootComponent`)) DeltaSeconds 10.0) false false)
    (`self.K2_AddActorLocalOffset` _returnvalue_2)
    (`self.K2_AddActorLocalOffset` (`self.Ship`) _returnvalue_2 false false)
    ;[1 1 1] Once we're finished moving, re-enable controls and stop the move
    (bind _output_get (set `self.TotalTravelDistance` (+ _returnvalue (`self.TotalTravelDistance`))))
    (if (>= _output_get (`self.VerticalDistance`))
      (set `self.IsFinishedMove` true)
      (`self.EnableInput` (`self.Ship`) (`GameplayStatics.GetPlayerController` 0))
      (`LightComponent.SetIntensity` (`self.PointLight`) 0.0))))

(event `self.TriggerBox.OnComponentBeginOverlap`
  (params (OverlappedComponent :type "PrimitiveComponent Object Reference") (OtherActor :type "Actor Object Reference") (OtherComp :type "PrimitiveComponent Object Reference") (OtherBodyIndex :type Integer) (bFromSweep :type Boolean) (SweepResult :type "HitResult Structure (by ref)"))
  (if (not (`self.IsFinishedMove`))
    (bind _asbp_ship (cast `/Game/FirstPersonBP/Blueprints/BP_Ship` OtherActor))
    (bind _output_get (set `self.Ship` _asbp_ship))
    (`self.DisableInput` _output_get (`GameplayStatics.GetPlayerController` 0))
    (set `self.PlayerInside` true)))

(fn `UserConstructionScript`)