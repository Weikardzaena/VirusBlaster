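; BP_LevelEndGate is a level exit gate that opens once all viruses in its linked RadarBounds are cleared.
; On BeginPlay it binds to the RadarBounds all-viruses-cleared event, and opens immediately when the FirstPersonGameMode's debug mode is on.
; Opening plays a timeline that lerps the actor upward by TravelDistance along Z from its current location.
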(event `self.ReceiveBeginPlay`
  (bind _asfirst_person_game_mode (cast `/Game/GameMode/FirstPersonGameMode` (`GameplayStatics.GetGameMode`)))
  (set `self.GameMode` _asfirst_person_game_mode)
  (if (`KismetSystemLibrary.IsValid` (`self.RadarBounds`))
    (add `/Game/Levels/RoomObjects/RadarLimitTrigger.OnAllVirusesCleared` (`self.RadarBounds`) (delegate `OnAllVirusesCleared`))
    (if (`/Game/GameMode/FirstPersonGameMode.DebugMode` (`self.GameMode`))
      (`self.OnAllVirusesCleared`))))

(event `OnAllVirusesCleared`
  (bind _returnvalue (`self.K2_GetActorLocation`))
  (set `self.StartingLocation` _returnvalue)
  (set `self.EndingLocation` (+ _returnvalue (`KismetMathLibrary.MakeVector` 0.0 0.0 (`self.TravelDistance`))))
  ;[1 1 1] Incrementally move gate in the +Z direction
  (bind (_direction _offset_timeline) (`Timeline|OpeningTimeline`)
    (:`Update`
      (`self.K2_SetActorLocation` (`KismetMathLibrary.VLerp` (`self.StartingLocation`) (`self.EndingLocation`) _offset_timeline)))))

(fn `UserConstructionScript`)