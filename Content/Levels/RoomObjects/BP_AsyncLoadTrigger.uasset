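; BP_AsyncLoadTrigger is a trigger that streams a named sublevel in and out as the ship enters and leaves its volume.
; On BeginPlay it binds begin and end overlap events on its CollisionComponent, both of which respond only to BP_Ship actors.
; Begin overlap loads LevelName without blocking and makes it visible once loaded, while end overlap unloads the same level.
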(event `self.ReceiveBeginPlay`
  (add `PrimitiveComponent.OnComponentBeginOverlap` (`self.CollisionComponent`) (delegate `OnComponentBeginOverlap`))
  (add `PrimitiveComponent.OnComponentEndOverlap` (`self.CollisionComponent`) (delegate `OnComponentEndOverlap_Event_0`)))

(event `OnComponentBeginOverlap`
  (params (OverlappedComponent :type "PrimitiveComponent Object Reference") (OtherActor :type "Actor Object Reference") (OtherComp :type "PrimitiveComponent Object Reference") (OtherBodyIndex :type Integer) (bFromSweep :type Boolean) (SweepResult :type "HitResult Structure (by ref)"))
  (cast `/Game/FirstPersonBP/Blueprints/BP_Ship` OtherActor)
  (`GameplayStatics.LoadStreamLevel` (`self.LevelName`) true))

(event `OnComponentEndOverlap_Event_0`
  (params (OverlappedComponent :type "PrimitiveComponent Object Reference") (OtherActor :type "Actor Object Reference") (OtherComp :type "PrimitiveComponent Object Reference") (OtherBodyIndex :type Integer))
  (cast `/Game/FirstPersonBP/Blueprints/BP_Ship` OtherActor)
  (`GameplayStatics.UnloadStreamLevel` (`self.LevelName`)))

(fn `UserConstructionScript`)